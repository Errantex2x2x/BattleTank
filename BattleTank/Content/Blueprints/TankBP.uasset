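; Player-controlled tank Blueprint that binds input to camera-rig aiming, movement and firing.
; On BeginPlay it hands the barrel and turret to TankAiming and both tracks to TankMovement.
; Aim axes yaw the azimuth gimbal and pitch the spring arm, scaled by delta time and speed.
; Opposing throttle axes are subtracted into turn and forward intents for TankMovement, while Fire calls TankAiming.
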(event `self.ReceiveBeginPlay`
  (`TankAimingComponent.Initialize` (`self.TankAiming`) (`self.TankBarrel`) (`self.TankTurret`))
  (`TankMovementComponent.Initialize` (`self.TankMovement`) (`self.TankTrackL`) (`self.TankTrackR`)))

(event `InputAction|Fire`
  (params (Key :type "Key Structure" :default "AnyKey"))
  (:`Pressed`
    (`TankAimingComponent.Fire` (`self.TankAiming`))))

(event `InputAxis|AimAzimuth`
  (params (AxisValue :type "Float (single-precision)"))
  ;[1 1 1] Input Aiming
  (`SceneComponent.K2_AddLocalRotation` (`self.Azimuth Gimbal`) (`KismetMathLibrary.MakeRotator` 0.0 0.0 (* AxisValue (`GameplayStatics.GetWorldDeltaSeconds`) (`self.AimAzimuthSpeed`))) false false))

(event `InputAxis|AimElevation`
  (params (AxisValue :type "Float (single-precision)"))
  ;[1 1 1] Input Aiming
  (`SceneComponent.K2_AddLocalRotation` (`self.SpringArm`) (`KismetMathLibrary.MakeRotator` 0.0 (* AxisValue (`GameplayStatics.GetWorldDeltaSeconds`) (`self.AimElevationSpeed`))) false false))

(event `InputAxis|RightThrottle`
  (params (AxisValue :type "Float (single-precision)"))
  ;[1 1 1] MovementInputBinding
  (`TankMovementComponent.IntendTurn` (`self.TankMovement`) (- (`self.GetInputAxisValue`) (`self.GetInputAxisValue`)) :!label _label))

(event `InputAxis|LeftThrottle`
  (params (AxisValue :type "Float (single-precision)"))
  ;[1 1 1] MovementInputBinding
  (goto _label))

(event `InputAxis|ForwardThrottle`
  (params (AxisValue :type "Float (single-precision)"))
  ;[1 1 1] MovementInputBinding
  (`TankMovementComponent.IntendMoveForward` (`self.TankMovement`) (- (`self.GetInputAxisValue`) (`self.GetInputAxisValue`)) :!label _label_2))

(event `InputAxis|BackwardsThrottle`
  (params (AxisValue :type "Float (single-precision)"))
  ;[1 1 1] MovementInputBinding
  (goto _label_2))

(fn `UserConstructionScript`)